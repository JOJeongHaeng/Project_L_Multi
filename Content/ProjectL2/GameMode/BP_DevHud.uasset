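; BP_DevHud is a HUD Blueprint that creates the HUD widget and feeds it player HP, boss HP and skill cooldowns.
; On BeginPlay it binds to event dispatchers on BP_PlayerState, BP_LGameState and BP_PlayerController, and pushes the current monster state as initial boss HP.
; Cooldown updates match the skill name in DT_Skills, using row index as widget slot and row CoolTime as maximum.
; The identity update handler is an empty stub.
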(event EventBeginPlay
  (bind _returnvalue (UserInterface|CreateWidget "/Game/UI/HudWidget.HudWidget_C"))
  (bind _output_get (Variables|Default|SetHudWidget _returnvalue))
  (UserInterface|Viewport|AddtoViewport _output_get 0)
  (CallFunction|BindPlayerState)
  (CallFunction|BindGameState)
  (bind _asbp_player_controller (Utilities|Casting|CastToBP_PlayerController (Game|GetPlayerController 0)))
  (EventDispatchers|BindEventtoUpdateSkillCool _asbp_player_controller (EventDispatchers|CreateEvent :!event UpdateCooltime))
  (EventDispatchers|BindEventtoUpdateIdentity _asbp_player_controller (EventDispatchers|CreateEvent :!event UpdateIdentity)))

(fn ConstructionScript)

(fn EventUpdateBossHp
  (params (CurHp :type Float%20%28double-precision%29) (MaxHp :type Float%20%28double-precision%29))
  (Default|SetBossHp (Variables|Default|GetHudWidget) CurHp MaxHp))

(fn BindPlayerState
  (bind _asbp_player_state (Utilities|Casting|CastToBP_PlayerState (Variables|/Script/Engine.Controller|GetPlayerState (Game|GetPlayerController 0))))
  (EventDispatchers|BindEventtoEventDispatcherUpdateHp _asbp_player_state (EventDispatchers|CreateEvent :!event EventUpdateHp)))

(fn EventUpdateHp
  (params (CurHp :type Float%20%28double-precision%29) (MaxHp :type Float%20%28double-precision%29))
  (Default|SetHp (Variables|Default|GetHudWidget) CurHp MaxHp))

(fn UpdateCooltime
  (params (SkillName :type String) (Cooltime :type Float%20%28double-precision%29))
  (LocalVariables|SetRemainCool Cooltime)
  (bind _outrownames (DataTable|GetDataTableRowNames "/Game/ProjectL/GameMode/Player/Skill/DT_Skills.DT_Skills"))
  (for (_array_element _array_index) _outrownames
    (bind _returnvalue (Utilities|GetDataTableRow "/Game/ProjectL/GameMode/Player/Skill/DT_Skills.DT_Skills" _array_element)
      (:then
        (if (Utilities|Enum|Equal(Enum) SkillName (.Name (Utilities|Struct|BreakST_Skill _returnvalue)))
          (Default|UpdateSkillCool (Variables|Default|GetHudWidget) (LocalVariables|GetRemainCool) (.CoolTime (Utilities|Struct|BreakST_Skill _returnvalue)) _array_index))))))

(fn UpdateIdentity
  (params (Identitycount :type Integer)))

(fn BindGameState
  (bind _asbp_dev_game_state (Utilities|Casting|CastToBP_LGameState (Game|GetGameState)))
  (EventDispatchers|BindEventtoEventDispatcherUpdateCurMonState _asbp_dev_game_state (EventDispatchers|CreateEvent :!event EventUpdatCurMonState))
  (CallFunction|EventUpdatCurMonState (Variables|/Game/ProjectL/GameMode/BP_LGameState.BP_LGameState_C|GetCur%20Mon%20State _asbp_dev_game_state)))

(fn EventUpdatCurMonState
  (params (CurMonStat :type ST%20Cur%20Mon%20State%20Structure))
  (Default|SetBossHp (Variables|Default|GetHudWidget) (.curhp CurMonStat) (.maxhp (.state CurMonStat))))