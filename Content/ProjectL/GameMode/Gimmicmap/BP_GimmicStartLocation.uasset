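; BP_GimmicStartLocation is a short-lived gimmick-map hazard that deals effectively lethal damage to any BP_LGamePawn beginning overlap with it.
; It destroys itself through a lifespan set on BeginPlay.
; While BP_LGameMode's Gimmic flag is set, Tick steadily shrinks its X/Y scale within clamped limits, keeps Z unchanged, and eases its location toward StartLoc with VInterpTo.
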(event EventBeginPlay
  (Actor|SetLifeSpan 11.0))

(event EventTick
  (params (DeltaSeconds :type Float%20%28single-precision%29))
  (CallFunction|GimmicStartMovement DeltaSeconds))

(event Collision|EventActorBeginOverlap
  (params (OtherActor :type Actor%20Object%20Reference))
  (bind _asbp_lgame_pawn (Utilities|Casting|CastToBP_LGamePawn OtherActor))
  (Game|Damage|ApplyDamage _asbp_lgame_pawn 5e+05 0 0))

(fn ConstructionScript)

(fn GimmicStartMovement
  (params (DeltaTime :type Float%20%28single-precision%29))
  (bind _returnvalue (Transformation|GetActorScale3D))
  (bind _returnvalue_2 (/ DeltaTime 1e+01))
  (bind _returnvalue_3 (* _returnvalue_2 55.0))
  (bind _asbp_lgame_mode (Utilities|Casting|CastToBP_LGameMode (Game|GetGameMode)))
  (if (Variables|/Game/ProjectL/GameMode/BP_LGameMode.BP_LGameMode_C|GetGimmic _asbp_lgame_mode)
    (Transformation|SetActorScale3D (Math|Vector|MakeVector (Math|Float|Clamp(Float) (- (.x _returnvalue) _returnvalue_3) 8.0 6e+01) (Math|Float|Clamp(Float) (- (.y _returnvalue) _returnvalue_3) 8.0 6e+01) (.z _returnvalue)))
    (Transformation|SetActorLocation (Math|Interpolation|VInterpTo (Transformation|GetActorLocation) (Variables|Default|GetStartLoc) DeltaTime 0.15) false false)))