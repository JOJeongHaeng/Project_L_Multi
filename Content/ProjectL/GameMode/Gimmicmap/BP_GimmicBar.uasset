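; BP_GimmicBar is a timed map hazard: a long cylinder bar that sweeps around the world origin and deals massive damage to any actor it overlaps.
; Tick calls TurnGimmicBar, which accumulates time and destroys the actor once its lifetime runs out.
; SinCosRadiusToLoc turns that time into a point on a fixed-radius circle in world space.
; An offset look-at rotation toward the origin lays the stretched cylinder flat along the radius.
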(event OnComponentBeginOverlap(Cylinder)
  (params (OverlappedComponent :type Primitive%20Component%20Object%20Reference) (OtherActor :type Actor%20Object%20Reference) (OtherComp :type Primitive%20Component%20Object%20Reference) (OtherBodyIndex :type Integer) (bFromSweep :type Boolean) (SweepResult :type Hit%20Result%20Structure%20%28by%20ref%29))
  (Game|Damage|ApplyDamage OtherActor 5e+05 0 0))

(event EventBeginPlay)

(event Collision|EventActorBeginOverlap
  (params (OtherActor :type Actor%20Object%20Reference)))

(event EventTick
  (params (DeltaSeconds :type Float%20%28single-precision%29))
  (if (> (Variables|Default|GetAddedTime) 25.0)
    (Actor|DestroyActor)
    (else
      (CallFunction|TurnGimmicBar DeltaSeconds))))

(fn ConstructionScript)

(fn TurnGimmicBar
  (params (Deltatime :type Float%20%28double-precision%29))
  (bind _output_get (Variables|Default|SetAddedTime (+ (Variables|Default|GetAddedTime) Deltatime)))
  (Transformation|SetWorldTransform (Variables|Default|GetCylinder) (Math|Transform|MakeTransform (CallFunction|SinCosRadiustoLoc (Math|Trig|DegreesToRadians (* _output_get 18.0)) 1e+03) (Math|Rotator|MakeRotator (+ (.Roll (Math|Rotator|BreakRotator (Math|Rotator|FindLookatRotation (CallFunction|SinCosRadiustoLoc (Math|Trig|DegreesToRadians (* _output_get 18.0)) 1e+03) (Math|Vector|MakeVectorNetQuantize 0.0 0.0 0.0)))) 9e+01) (.Pitch (Math|Rotator|BreakRotator (Math|Rotator|FindLookatRotation (CallFunction|SinCosRadiustoLoc (Math|Trig|DegreesToRadians (* _output_get 18.0)) 1e+03) (Math|Vector|MakeVectorNetQuantize 0.0 0.0 0.0)))) (+ (.Yaw (Math|Rotator|BreakRotator (Math|Rotator|FindLookatRotation (CallFunction|SinCosRadiustoLoc (Math|Trig|DegreesToRadians (* _output_get 18.0)) 1e+03) (Math|Vector|MakeVectorNetQuantize 0.0 0.0 0.0)))) 9e+01)) "1.000000,1.000000,13.000000") false false))

(fn SinCosRadiustoLoc
  (params (Degree :type Float%20%28double-precision%29) (Raidus :type Float%20%28double-precision%29))
  (return (Math|Vector|MakeVector (* (Math|Trig|Sin(Radians) Degree) Raidus) (* (Math|Trig|Cos(Radians) Degree) Raidus) 1e+02)))