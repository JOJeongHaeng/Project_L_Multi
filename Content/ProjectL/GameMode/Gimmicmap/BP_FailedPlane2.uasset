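; BP_FailedPlane2 is a damage floor hazard for a gimmick map.
; Begin and end overlap events set a flag while a BP_LGamePawn is on the plane.
; Each Tick, ApplyDamageForTime accumulates delta time while flagged and, past a half-second interval, applies heavy damage to player 0's controlled pawn rather than the overlapping actor, then resets the timer.
; Debug strings print on overlap and damage.
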(event EventBeginPlay)

(event EventTick
  (params (DeltaSeconds :type Float%20%28single-precision%29))
  (CallFunction|ApplyDamageforTime DeltaSeconds))

(event Collision|EventActorBeginOverlap
  (params (OtherActor :type Actor%20Object%20Reference))
  (Development|PrintString "overlapSuc")
  (Utilities|Casting|CastToBP_LGamePawn OtherActor)
  (Variables|Default|SetOverlaped true))

(event Collision|EventActorEndOverlap
  (params (OtherActor :type Actor%20Object%20Reference))
  (Development|PrintString "overlapEndSuc")
  (Utilities|Casting|CastToBP_LGamePawn OtherActor)
  (Variables|Default|SetOverlaped false))

(fn ConstructionScript)

(fn ApplyDamageforTime
  (params (A :type Float%20%28double-precision%29))
  (if (Variables|Default|GetOverlaped)
    (Variables|Default|SetTime (+ A (Variables|Default|GetTime)))
    (if (> (Variables|Default|GetTime) 0.5)
      (bind _returnvalue (Game|Damage|ApplyDamage (Pawn|GetControlledPawn (Game|GetPlayerController 0)) 1e+03 0 0))
      (Development|PrintString (Utilities|String|Append "Damage floor" (Utilities|String|ToString(Float) _returnvalue)))
      (Variables|Default|SetTime 0.0))))