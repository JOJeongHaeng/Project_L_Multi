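; Gimmick-map actor that spawns a ring of eight BP_GimmicBall2 actors when play begins.
; BeginPlay calls InitializeBallsLocation, which stores the radius and spawns the balls at 45-degree intervals through unrolled spawn calls.
; SinCoswithRadius converts each angle and the radius into a position at fixed height, so the ring centers on the world origin, independent of this actor's location.
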(event EventBeginPlay
  (CallFunction|InitializeBallsLocation 1.5e+03))

(event Collision|EventActorBeginOverlap
  (params (OtherActor :type Actor%20Object%20Reference)))

(event EventTick
  (params (DeltaSeconds :type Float%20%28single-precision%29)))

(fn ConstructionScript)

(fn InitializeBallsLocation
  (params (Rad :type Float%20%28double-precision%29))
  (LocalVariables|SetRadius Rad)
  (Game|SpawnActorfromClass "/Game/ProjectL/GameMode/Gimmicmap/BP_GimmicBall2.BP_GimmicBall2_C" (Math|Transform|MakeTransform (CallFunction|SinCoswithRadius (Math|Trig|DegreesToRadians 0.0) (LocalVariables|GetRadius)) "0, 0, 0" "1.000000,1.000000,1.000000") "Undefined" "MultiplyWithRoot" 0 0)
  (Game|SpawnActorfromClass "/Game/ProjectL/GameMode/Gimmicmap/BP_GimmicBall2.BP_GimmicBall2_C" (Math|Transform|MakeTransform (CallFunction|SinCoswithRadius (Math|Trig|DegreesToRadians 45.0) (LocalVariables|GetRadius)) "0, 0, 0" "1.000000,1.000000,1.000000") "Undefined" "MultiplyWithRoot" 0 0)
  (Game|SpawnActorfromClass "/Game/ProjectL/GameMode/Gimmicmap/BP_GimmicBall2.BP_GimmicBall2_C" (Math|Transform|MakeTransform (CallFunction|SinCoswithRadius (Math|Trig|DegreesToRadians 9e+01) (LocalVariables|GetRadius)) "0, 0, 0" "1.000000,1.000000,1.000000") "Undefined" "MultiplyWithRoot" 0 0)
  (Game|SpawnActorfromClass "/Game/ProjectL/GameMode/Gimmicmap/BP_GimmicBall2.BP_GimmicBall2_C" (Math|Transform|MakeTransform (CallFunction|SinCoswithRadius (Math|Trig|DegreesToRadians 135.0) (LocalVariables|GetRadius)) "0, 0, 0" "1.000000,1.000000,1.000000") "Undefined" "MultiplyWithRoot" 0 0)
  (Game|SpawnActorfromClass "/Game/ProjectL/GameMode/Gimmicmap/BP_GimmicBall2.BP_GimmicBall2_C" (Math|Transform|MakeTransform (CallFunction|SinCoswithRadius (Math|Trig|DegreesToRadians 1.8e+02) (LocalVariables|GetRadius)) "0, 0, 0" "1.000000,1.000000,1.000000") "Undefined" "MultiplyWithRoot" 0 0)
  (Game|SpawnActorfromClass "/Game/ProjectL/GameMode/Gimmicmap/BP_GimmicBall2.BP_GimmicBall2_C" (Math|Transform|MakeTransform (CallFunction|SinCoswithRadius (Math|Trig|DegreesToRadians 225.0) (LocalVariables|GetRadius)) "0, 0, 0" "1.000000,1.000000,1.000000") "Undefined" "MultiplyWithRoot" 0 0)
  (Game|SpawnActorfromClass "/Game/ProjectL/GameMode/Gimmicmap/BP_GimmicBall2.BP_GimmicBall2_C" (Math|Transform|MakeTransform (CallFunction|SinCoswithRadius (Math|Trig|DegreesToRadians 2.7e+02) (LocalVariables|GetRadius)) "0, 0, 0" "1.000000,1.000000,1.000000") "Undefined" "MultiplyWithRoot" 0 0)
  (Game|SpawnActorfromClass "/Game/ProjectL/GameMode/Gimmicmap/BP_GimmicBall2.BP_GimmicBall2_C" (Math|Transform|MakeTransform (CallFunction|SinCoswithRadius (Math|Trig|DegreesToRadians 315.0) (LocalVariables|GetRadius)) "0, 0, 0" "1.000000,1.000000,1.000000") "Undefined" "MultiplyWithRoot" 0 0))

(fn SinCoswithRadius
  (params (dig :type Float%20%28double-precision%29) (Rad :type Float%20%28double-precision%29))
  (return (Math|Vector|MakeVector (* (Math|Trig|Sin(Radians) dig) Rad) (* (Math|Trig|Cos(Radians) dig) Rad) 1e+02)))