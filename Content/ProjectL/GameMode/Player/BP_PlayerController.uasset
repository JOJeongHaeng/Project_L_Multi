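; Player controller for BP_LGamePawn, providing cursor-based click-to-move, server-side attack damage boxes and an identity skill.
; Server events update identity on BP_PlayerState and spawn a DamageBox ahead of the pawn, passing its current montage.
; Tick polls the player state for death, then flags it and ragdolls the pawn mesh.
; Init enables mouse interaction and binds damage handling, while BossDie notifies the HUD widget.
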(event Custom|SeverUseIdentity
  (bind _asbp_player_state (Utilities|Casting|CastToBP_PlayerState (Variables|Default|GetPlayerState)))
  (Default|UpdateIdentity _asbp_player_state 1))

(event Custom|ServerSpawnDamagebox
  (params (Animation :type Anim%20Sequence%20Base%20Object%20Reference))
  (CallFunction|ServerSpawn))

(event EventBeginPlay
  ;[0.15 0.15 0.15 0.5] mouse 보이게 + click event
  (CallFunction|Init))

(event EventTick
  (params (DeltaSeconds :type Float%20%28single-precision%29))
  ;[0.15 0.15 0.15 0.5] 마우스 input 으로 움직임 구현
  (Utilities|FlowControl|Sequence
    (:then_0
      (Variables|Default|SetbCanMove (Variables|Default|GetCanMove)))
    (:then_1
      (bind _asbp_player_state (Utilities|Casting|CastToBP_PlayerState (Variables|Default|GetPlayerState)))
      (if (Default|IsDeath _asbp_player_state)
        (Variables|Default|SetIsDead true)
        (bind _asbp_lgame_pawn (Utilities|Casting|CastToBP_LGamePawn (Pawn|GetControlledPawn)))
        (Physics|SetSimulatePhysics (Variables|/Script/Engine.Character|GetMesh _asbp_lgame_pawn) true)))))

(fn ConstructionScript)

(fn MouseClickMoveMent
  (bind _hitresult (Game|Player|GetHitResultUnderCursorbyChannel "TraceTypeQuery1" true))
  (bind _location (Collision|BreakHitResult _hitresult))
  (bind (_x _y) (Math|Vector|BreakVector _location))
  (if (Variables|Default|GetCanMove)
    (Utilities|Casting|CastToBP_LGamePawn (Pawn|GetControlledPawn))
    (Rendering|Debug|DrawDebugSphere _location 1e+02 12 "(R=1.000000,G=0.024480,B=0.000000,A=1.000000)" 0.0)
    (AI|Navigation|SimpleMovetoLocation self (Math|Vector|MakeVector _x _y 0.0))))

(fn SpawnDamageBox
  (params (Animation :type Anim%20Sequence%20Base%20Object%20Reference))
  (CallFunction|ServerSpawnDamagebox Animation))

(fn Init
  (Variables|Default|SetbShowMouseCursor true)
  (Variables|Default|SetbEnableClickEvents true)
  (Variables|Default|SetbEnableMouseOverEvents true)
  ;[0.15 0.15 0.15 0.5] Serverbind
  (EventDispatchers|BindEventtoApplyDamage (EventDispatchers|CreateEvent :!event SpawnDamageBox)))

(fn CanUseIdentity
  (bind _asbp_player_state (Utilities|Casting|CastToBP_PlayerState (Variables|Default|GetPlayerState))
    (:then
      (if (Default|CanuseIdentity _asbp_player_state)
        (return true)
        (else
          (return false))))
    (:CastFailed
      (Development|PrintString "Controller to StateCastFailed"))))

(fn CallServerIdentity
  (Networking|SwitchHasAuthority
    (:Authority
      (Development|PrintString "server use identity"))
    (:Remote
      (Development|PrintString "client use identity")))
  (CallFunction|SeverUseIdentity))

(fn ServerSpawn
  (bind _returnvalue (Pawn|GetControlledPawn))
  (bind _returnvalue_2 (Transformation|GetActorForwardVector _returnvalue))
  (bind _returnvalue_3 (Math|Rotator|MakeRotfromX _returnvalue_2))
  (Networking|SwitchHasAuthority
    (:Authority
      (bind _asbp_lgame_pawn (Utilities|Casting|CastToBP_LGamePawn _returnvalue))
      (Game|SpawnActorfromClass "/Game/ProjectL/GameMode/Player/Skill/Damage/DamageBox.DamageBox_C" (Math|Transform|MakeTransform (+ (Transformation|GetActorLocation _returnvalue) (* _returnvalue_2 2.7e+02)) (Math|Rotator|MakeRotator (.roll _returnvalue_3) (.pitch _returnvalue_3) (+ (.yaw _returnvalue_3) 9e+01)) "1.000000,1.000000,1.000000") "Undefined" "MultiplyWithRoot" self (Animation|GetCurrentMontage _asbp_lgame_pawn :!class /Script/Engine.Character) 0))))

(fn BossDie
  (bind _asbp_hud (Utilities|Casting|CastToBP_Hud (HUD|GetHUD)))
  (Default|BossDie (Variables|/Game/UI/BP_Hud.BP_Hud_C|GetHudWidget _asbp_hud)))