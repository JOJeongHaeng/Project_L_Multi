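; Skill component for BP_LGamePawn that runs data-driven skills with cooldowns and an optional identity cost.
; On BeginPlay it builds SkillArr from DT_Skills and starts a looping one-second timer that decrements active cooldowns and reports them to BP_PlayerController.
; UseSkill checks cooldown, spends identity through the controller if required, resets cooldown from the table, disables movement and plays the montage, returning its result and the controller.
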(event EventBeginPlay
  (CallFunction|InitializeSkillArr)
  (Utilities|Time|SetTimerbyFunctionName 0 "UpdateSkillCoolTime" 1.0 true))

(fn UseSkill
  (params (RowName :type Name))
  (bind _returnvalue (Utilities|GetDataTableRow "/Game/ProjectL/GameMode/Player/Skill/DT_Skills.DT_Skills" RowName)
    (:then
      (for (_array_element _array_index) (Variables|Default|GetSkillArr)
        (if (Utilities|Enum|Equal(Enum) (.Name (Utilities|Struct|BreakST_Skill _array_element)) (.Name (Utilities|Struct|BreakST_Skill _returnvalue)))
          (if (<= (.CoolTime (Utilities|Struct|BreakST_Skill _array_element)) 0.0)
            (if (.UseIdentity (Utilities|Struct|BreakST_Skill _returnvalue))
              (bind _asbp_lgame_pawn (Utilities|Casting|CastToBP_LGamePawn (Components|GetOwner)))
              ;[0.15 0.15 0.15 0.5] identity 스킬 사용가능여부 확인후 사용
              (bind _asbp_player_controller (Utilities|Casting|CastToBP_PlayerController (Pawn|GetController _asbp_lgame_pawn)))
              (bind _canuse (Default|CanUseIdentity _asbp_player_controller))
              (if _canuse
                (Default|CallUpdateIdentity _asbp_player_controller -1)
                ;[0.15 0.15 0.15 0.5] skill 사용후 다시 쿨타임을원복
                (bind _structout (Utilities|Struct|SetmembersinST_Skill _array_element :!label _label))
                (Utilities|Array|SetArrayElem (Variables|Default|GetSkillArr) _array_index (Utilities|Struct|MakeST_Skill (.name _structout) (.animmontage _structout) (.CoolTime (Utilities|Struct|BreakST_Skill _returnvalue)) (.useidentity _structout) (.chargeidentity _structout) (.damage _structout) (.damagesize _structout)))
                (bind _asbp_lgame_pawn_2 (Utilities|Casting|CastToBP_LGamePawn (Components|GetOwner)))
                ;[0.15 0.15 0.15 0.5] 애니메이션 실행
                (bind _asbp_player_controller_2 (Utilities|Casting|CastToBP_PlayerController (Pawn|GetController _asbp_lgame_pawn_2))
                  (:then
                    (Variables|/Game/ProjectL/GameMode/Player/BP_PlayerController.BP_PlayerController_C|SetCanMove _asbp_player_controller_2 false)
                    (bind _asbp_lgame_pawn_3 (Utilities|Casting|CastToBP_LGamePawn (Components|GetOwner))
                      (:then
                        (bind _returnvalue_2 (Animation|PlayAnimMontage _asbp_lgame_pawn_3 (.AnimMontage (Utilities|Struct|BreakST_Skill _array_element)) 1.0 "None"))
                        (return _returnvalue_2 _asbp_player_controller_2))
                      (:CastFailed
                        ;[0.15 0.15 0.15 0.5] Debug
                        (Development|PrintString "UseSkillFunOwnerFailed"))))
                  (:CastFailed
                    ;[0.15 0.15 0.15 0.5] Debug
                    (Development|PrintString "UseSkillFunController")))
                (else
                  (Development|PrintString "Cantuseidentity skill")))
              (else
                (goto _label)))
            (else
              ;[0.15 0.15 0.15 0.5] debug
              (Development|PrintString "Skill Is CoolTime")
              (return -1.0 0))))))
    (:RowNotFound
      ;[0.15 0.15 0.15 0.5] Debug
      (Development|PrintString "UseSkillFunRowNotFound"))))

(fn InitializeSkillArr
  (bind _outrownames (DataTable|GetDataTableRowNames "/Game/ProjectL/GameMode/Player/Skill/DT_Skills.DT_Skills"))
  (for _array_element _outrownames
    (bind _returnvalue (Utilities|GetDataTableRow "/Game/ProjectL/GameMode/Player/Skill/DT_Skills.DT_Skills" _array_element)
      (:then
        (Utilities|Array|Add (Variables|Default|GetSkillArr) (Utilities|Struct|MakeST_Skill (.Name (Utilities|Struct|BreakST_Skill _returnvalue)) (.AnimMontage (Utilities|Struct|BreakST_Skill _returnvalue)) 0.0 (.UseIdentity (Utilities|Struct|BreakST_Skill _returnvalue)) (.ChargeIdentity (Utilities|Struct|BreakST_Skill _returnvalue)))))
      (:RowNotFound
        (Development|PrintString "RowNotFound")))))

(fn UpdateSkillCoolTime
  (for (_array_element _array_index) (Variables|Default|GetSkillArr)
    (if (> (.CoolTime (Utilities|Struct|BreakST_Skill _array_element)) 0.0)
      (bind _structout (Utilities|Struct|SetmembersinST_Skill _array_element))
      (Utilities|Array|SetArrayElem (Variables|Default|GetSkillArr) _array_index (Utilities|Struct|MakeST_Skill (.name _structout) (.animmontage _structout) (Utilities|Operators|Subtract (.cooltime _structout) 1.0) (.useidentity _structout) (.chargeidentity _structout) (.damage _structout) (.damagesize _structout)))
      (bind _asbp_lgame_pawn (Utilities|Casting|CastToBP_LGamePawn (Components|GetOwner)))
      (bind _asbp_player_controller (Utilities|Casting|CastToBP_PlayerController (Pawn|GetController _asbp_lgame_pawn)))
      (Default|CallUpdateSkillCool _asbp_player_controller (.Name (Utilities|Struct|BreakST_Skill _array_element)) (.CoolTime (Utilities|Struct|BreakST_Skill _array_element)))))
  ;[0.15 0.15 0.15 0.5] Debug
  (Development|PrintString "CoolTime -1 "))