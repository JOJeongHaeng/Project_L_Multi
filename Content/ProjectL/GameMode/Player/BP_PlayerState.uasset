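; BP_PlayerState holds a player's HP, stun state and clamped Identity counter, which gates identity use.
; Server-only AddDamage lowers HP and fires HP and death dispatchers, while Tick flags death on BP_LGameMode.
; Tick also runs a server-side timed stun that spawns BP_Stun and blocks movement, always targeting player controller 0.
; Identity changes come through a BP_PlayerController binding and reach BP_Hud directly and via OnRep.
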(event EventBeginPlay
  (bind _asbp_player_controller (Utilities|Casting|CastToBP_PlayerController (Components|GetOwner)))
  (EventDispatchers|BindEventtoUpdateIdentity _asbp_player_controller (EventDispatchers|CreateEvent :!event UpdateIdentity)))

(event EventTick
  (params (DeltaSeconds :type Float%20%28single-precision%29))
  (Utilities|FlowControl|Sequence
    (:then_0
      (CallFunction|Stun DeltaSeconds))
    (:then_1
      (CallFunction|PlayerDie))))

(fn ConstructionScript)

(fn UpdateIdentity
  (params (updateCount :type Integer))
  (bind _output_get (Variables|Default|SetIdentity (Math|Integer|Clamp(Integer) (+ updateCount (Variables|Default|GetIdentity)) 0 2)))
  (bind _asbp_player_controller (Utilities|Casting|CastToBP_PlayerController (Components|GetOwner)))
  (bind _asbp_hud (Utilities|Casting|CastToBP_Hud (HUD|GetHUD _asbp_player_controller)))
  (Default|SetIdentity (Variables|/Game/UI/BP_Hud.BP_Hud_C|GetHudWidget _asbp_hud) _output_get))

(fn Stun
  (params (B :type Float%20%28double-precision%29))
  (Networking|SwitchHasAuthority
    (:Authority
      (if (Variables|Default|GetIsStun)
        (Variables|Default|SetStunTime (+ (Variables|Default|GetStunTime) B))
        (if (Variables|Default|GetStunActorSpawned)
          _
          (else
            ;[0.15 0.15 0.15 0.5] 고칠부분(완료)
            (bind _asbp_lgame_pawn (Utilities|Casting|CastToBP_LGamePawn (Pawn|GetControlledPawn (Game|GetPlayerController 0))))
            (Game|SpawnActorfromClass "/Game/ProjectL/GameMode/Player/Character/PlayerState/BP_Stun.BP_Stun_C" (Math|Transform|MakeTransform (Math|Vector|MakeVector (.x (.location (Transformation|GetActorTransform _asbp_lgame_pawn))) (.y (.location (Transformation|GetActorTransform _asbp_lgame_pawn))) 2e+02) (.rotation (Transformation|GetActorTransform _asbp_lgame_pawn)) "1.000000,1.000000,1.000000") "Undefined" "MultiplyWithRoot" 0 0)
            (Variables|Default|SetStunActorSpawned true)))
        (if (> (Variables|Default|GetStunTime) 1.0)
          (Variables|Default|SetStunTime 0.0)
          (bind _asbp_player_controller (Utilities|Casting|CastToBP_PlayerController (Game|GetPlayerController 0))
            (:then
              (Variables|/Game/ProjectL/GameMode/Player/BP_PlayerController.BP_PlayerController_C|SetCanMove _asbp_player_controller true)
              (Variables|Default|SetIsStun false)
              (Variables|Default|SetStunActorSpawned false))
            (:CastFailed
              (Development|PrintString "cast failed")))
          (else
            (bind _asbp_player_controller_2 (Utilities|Casting|CastToBP_PlayerController (Game|GetPlayerController 0))
              (:then
                (Variables|/Game/ProjectL/GameMode/Player/BP_PlayerController.BP_PlayerController_C|SetCanMove _asbp_player_controller_2 false))
              (:CastFailed
                (Development|PrintString "cast failed")))))))))

(fn AddDamage
  (params (Damage :type Float%20%28double-precision%29))
  (Networking|SwitchHasAuthority
    (:Authority
      (Development|PrintString "Damaged!")
      (bind _output_get (Variables|Default|SetCurHp (- (Variables|Default|GetCurHp) Damage)))
      (Default|CallEventDispatcherUpdateHp _output_get (Variables|Default|GetMaxHp))
      (if (<= (Variables|Default|GetCurHp) 0.0)
        (Default|CallEventDispatcherDeath)))))

(fn IsDeath
  (return (<= (Variables|Default|GetCurHp) 0.0)))

(fn PlayerDie
  (if (<= (Variables|Default|GetCurHp) 0.0)
    (bind _asbp_lgame_mode (Utilities|Casting|CastToBP_LGameMode (Game|GetGameMode)))
    (Variables|/Game/ProjectL/GameMode/BP_LGameMode.BP_LGameMode_C|SetPlayerDied _asbp_lgame_mode true)))

(fn OnRepCurHp)

(fn OnRepMaxHp)

(fn OnRepIdentity
  (Development|PrintString "onrepidentity")
  (bind _asbp_player_controller (Utilities|Casting|CastToBP_PlayerController (Components|GetOwner)))
  (bind _asbp_hud (Utilities|Casting|CastToBP_Hud (HUD|GetHUD _asbp_player_controller)))
  (Default|UpdateIdentity _asbp_hud (Variables|Default|GetIdentity)))

(fn OnRepIsStun)

(fn CanuseIdentity
  (if (> (Variables|Default|GetIdentity) 0)
    (return true)
    (else
      (return false))))