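; BP_DamageActor is a short-lived floating damage number shown in the world through a widget component.
; On BeginPlay it passes its damage value and text color to the DamageWidget, then expires after two seconds.
; Each tick the widget tracks the Instigator's horizontal position, rises at a constant frame-rate-independent speed and rotates to face the player camera.
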(event EventBeginPlay
  (bind _asdamage_widget (Utilities|Casting|CastToDamageWidget (UserInterface|GetUserWidgetObject (Variables|Default|GetWidget))))
  (Default|UpdateDamage _asdamage_widget (Variables|Default|GetDamage))
  (Default|UpdateColor _asdamage_widget (Variables|Default|GetTextColor))
  (Actor|SetLifeSpan 2.0))

(event EventTick
  (params (DeltaSeconds :type Float%20%28single-precision%29))
  (CallFunction|DamagelocandRot DeltaSeconds))

(fn ConstructionScript)

(fn DamagelocandRot
  (params (A :type Float%20%28double-precision%29))
  (bind _widget (Variables|Default|GetWidget))
  (bind _instigator (Variables|Actor|GetInstigator))
  (bind _returnvalue (Transformation|GetActorTransform _instigator))
  (Transformation|SetWorldLocationAndRotation _widget (Math|Vector|MakeVector (.x (.location _returnvalue)) (.y (.location _returnvalue)) (+ (* A 5e+01) (.z (Transformation|GetWorldLocation (Variables|Default|GetWidget))))) (Math|Rotator|FindLookatRotation (Transformation|GetWorldLocation _widget) (Camera|GetCameraLocation (Game|GetPlayerCameraManager 0))) false false))