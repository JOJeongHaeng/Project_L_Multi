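; BP_Camera is a gameplay camera that becomes player 0's view target on BeginPlay and keeps the world origin in view.
; Each tick it aims at the origin and sits at a fixed height along the horizontal line from the origin through the controlled BP_LGamePawn's mesh.
; Its radius from the origin grows in small per-frame steps when the pawn is too close, otherwise shrinks toward a minimum, without delta-time scaling.
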(event EventBeginPlay
  (Game|Player|SetViewTargetwithBlend (Game|GetPlayerController 0) self 0.0 "VTBlend_Linear" 0.0 false))

(event Collision|EventActorBeginOverlap
  (params (OtherActor :type Actor%20Object%20Reference)))

(event EventTick
  (params (DeltaSeconds :type Float%20%28single-precision%29))
  (CallFunction|TickCameraPos))

(fn ConstructionScript)

(fn TickCameraPos
  (Transformation|SetWorldRotation (Variables|CameraActor|GetCameraComponent) (Math|Rotator|FindLookatRotation (Transformation|GetWorldLocation (Variables|CameraActor|GetCameraComponent)) (Math|Vector|MakeVectorNetQuantize 0.0 0.0 0.0)) false false)
  (bind _asbp_lgame_pawn (Utilities|Casting|CastToBP_LGamePawn (Pawn|GetControlledPawn (Game|GetPlayerController 0))))
  (if (< (Math|Vector|Distance(Vector) (Transformation|GetWorldLocation (Variables|CameraActor|GetCameraComponent)) (Transformation|GetWorldLocation (Variables|/Script/Engine.Character|GetMesh _asbp_lgame_pawn))) 2e+03)
    (Variables|Default|SetCameraLength (+ (Variables|Default|GetCameraLength) 3.0))
    (elif (>= (Variables|Default|GetCameraLength) 3.7e+03)
      (Variables|Default|SetCameraLength (- (Variables|Default|GetCameraLength) 3.0))))
  (Transformation|SetWorldLocation (Variables|CameraActor|GetCameraComponent) (Math|Vector|MakeVector (* (.x (Math|Vector|Normalize (Math|Vector|MakeVector (.x (Transformation|GetWorldLocation (Variables|/Script/Engine.Character|GetMesh _asbp_lgame_pawn))) (.y (Transformation|GetWorldLocation (Variables|/Script/Engine.Character|GetMesh _asbp_lgame_pawn))) 0.0) 1.0)) (Variables|Default|GetCameraLength)) (* (.y (Math|Vector|Normalize (Math|Vector|MakeVector (.x (Transformation|GetWorldLocation (Variables|/Script/Engine.Character|GetMesh _asbp_lgame_pawn))) (.y (Transformation|GetWorldLocation (Variables|/Script/Engine.Character|GetMesh _asbp_lgame_pawn))) 0.0) 1.0)) (Variables|Default|GetCameraLength)) 1.5e+03) false false))