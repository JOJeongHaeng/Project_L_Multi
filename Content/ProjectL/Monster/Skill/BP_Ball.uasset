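; BP_Ball is a monster-skill rock projectile that stuns and damages the player pawn it overlaps.
; On spawn it scales up, lifts itself, snapshots player 0's location through BP_PlayerController and sets a short lifespan.
; Each tick it eases toward that fixed point with VInterpTo while tumbling.
; Overlaps are handled on authority only, setting the stun flag on BP_PlayerState and applying damage to BP_LGamePawn.
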(event EventBeginPlay
  (bind _returnvalue (Transformation|GetActorLocation))
  (Transformation|SetActorScale3D "2.000000,2.000000,2.000000")
  (Transformation|SetActorLocation (Math|Vector|MakeVector (.x _returnvalue) (.y _returnvalue) (+ (.z _returnvalue) 3e+02)) false false)
  (Variables|Default|SetDestinationLoc (CallFunction|FindPlayerLoc))
  (Actor|SetLifeSpan 1.0))

(event EventTick
  (params (DeltaSeconds :type Float%20%28single-precision%29))
  (bind _returnvalue (Transformation|GetActorRotation))
  (Transformation|SetActorLocation (Math|Interpolation|VInterpTo (Transformation|GetActorLocation) (Variables|Default|GetDestinationLoc) DeltaSeconds 2.5) false false)
  (Transformation|SetActorRotation (Math|Rotator|MakeRotator (+ (.roll _returnvalue) 5.0) (+ (.pitch _returnvalue) 3.0) (+ (.yaw _returnvalue) 1.0))))

(event Collision|EventActorBeginOverlap
  (params (OtherActor :type Actor%20Object%20Reference))
  (Networking|SwitchHasAuthority
    (:Authority
      (bind _asbp_lgame_pawn (Utilities|Casting|CastToBP_LGamePawn OtherActor)
        (:then
          (bind _asbp_player_state (Utilities|Casting|CastToBP_PlayerState (Variables|/Script/Engine.Pawn|GetPlayerState _asbp_lgame_pawn))
            (:then
              (Variables|/Game/ProjectL/GameMode/Player/BP_PlayerState.BP_PlayerState_C|SetISStun _asbp_player_state true)
              (Game|Damage|ApplyDamage _asbp_lgame_pawn 1e+03 0 0))
            (:CastFailed
              (Development|PrintString "Rock Cast failed" :!label _label))))
        (:CastFailed
          (goto _label))))))

(fn ConstructionScript)

(fn FindPlayerLoc
  (bind _asbp_player_controller (Utilities|Casting|CastToBP_PlayerController (Game|GetPlayerController 0)))
  (bind _returnvalue (Default|ReturnPlayerLoc _asbp_player_controller))
  (return _returnvalue))