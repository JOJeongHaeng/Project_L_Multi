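; BP_BossSkillMgr is a manager for boss monster skills, currently an unfinished skeleton.
; Each Tick, UpdateSkills loops over the Skills array and passes every entry with delta time to UpdateSkillCoolTime.
; That function is empty: its logic to accumulate time, fire the skill past its data cooldown and reset is disconnected and never runs.
; DoUseSkill is also an empty stub, so no skill executes.
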(event EventTick
  (params (DeltaSeconds :type Float%20%28single-precision%29))
  (CallFunction|UpdateSkills DeltaSeconds))

(fn UpdateSkills
  (params (DeltaSeconds :type Float%20%28double-precision%29))
  (for (_ _array_index) (Variables|Default|GetSkills)
    (CallFunction|UpdateSkillCoolTime (Utilities|Array|Get(acopy) (Variables|Default|GetSkills) _array_index) DeltaSeconds)))

(fn UpdateSkillCoolTime
  (params (CurSkill :type ST%20Cur%20Boss%20Skill%20Structure) (DeltaSeconds :type Float%20%28double-precision%29)))

(fn DoUseSkill
  (params (CurSkill :type ST%20Cur%20Boss%20Skill%20Structure)))